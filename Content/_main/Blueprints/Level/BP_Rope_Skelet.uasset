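; Skeletal-mesh physics rope that the player character can grab, swing on, climb and launch off.
; Overlap notifies the character; grabbing hangs it from the massed bone nearest its head, found via per-bone boxes built at construction, and pushes that bone forward.
; Swing input adds force to the active bone, while climbing shifts it along a clamped bone range.
; Release restores walking and launches the character with doubled bone velocity.
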(event Custom|Climb
  (params (ClimbDirection :type Float%20%28double-precision%29))
  (if (not (Variables|Default|GetIsClimbing?))
    (bind _output_get (Variables|Default|SetClimbDirection ClimbDirection))
    (bind _climb_ (CallFunction|CanClimb? _output_get))
    (if _climb_
      (Variables|Default|SetIsClimbing? true)
      (if (> (Variables|Default|GetClimbDirection) 0.0)
        (Default|ClimbRope (Variables|Default|GetCharRef))))))

(event Custom|AddSwingForce
  (params (SwingForce :type Vector))
  ;[1 1 1] Swinging
  (if (not (Variables|Default|GetIsClimbing?))
    (Physics|AddForce (Variables|Default|GetRope_Mesh) (* SwingForce 5e+02) (Variables|Default|GetActiveRopeBone) true)))

(event EventBeginPlay
  (Actor|Tick|SetActorTickEnabled false))

(event Collision|EventActorBeginOverlap
  (params (OtherActor :type Actor%20Object%20Reference))
  (bind _isplayer_ (Class|BPIPlayerRef|IsPlayer?(Message) OtherActor))
  (if _isplayer_
    (bind _asbp_third_person_character (Utilities|Casting|CastToBP_ThirdPersonCharacter OtherActor))
    (if (not (Variables|/Game/ThirdPerson/Blueprints/BP_ThirdPersonCharacter.BP_ThirdPersonCharacter_C|GetIsOnRope? _asbp_third_person_character))
      (Default|FindRope _asbp_third_person_character)
      (Actor|Tick|SetActorTickEnabled true))))

(event EventAttatchtoRope
  (params (CharRef :type BP%20Third%20Person%20Character%20Object%20Reference))
  ;[1 1 1] Grab a Rope
  (Variables|Default|SetCharRef CharRef)
  (bind _closestindex (CallFunction|FindBestBone))
  (bind _output_get (Variables|Default|SetActiveRopeBone (Class|SkinnedMeshComponent|GetBoneName (Variables|Default|GetRope_Mesh) _closestindex)))
  (Default|Hang (Variables|Default|GetCharRef) self _output_get)
  (Physics|SetPhysicsLinearVelocity (Variables|Default|GetRope_Mesh) (* (Variables|Default|GetInitialVelocity) (Transformation|GetActorForwardVector (Variables|Default|GetCharRef))) false (Variables|Default|GetActiveRopeBone)))

(event Collision|EventActorEndOverlap
  (params (OtherActor :type Actor%20Object%20Reference))
  (bind _isplayer_ (Class|BPIPlayerRef|IsPlayer?(Message) OtherActor))
  (if _isplayer_
    (Utilities|Casting|CastToBP_ThirdPersonCharacter OtherActor)
    (Actor|Tick|SetActorTickEnabled false)))

(event EventUnhold
  (params (CharRef :type Character%20Object%20Reference))
  (bind _asbp_third_person_character (Utilities|Casting|CastToBP_ThirdPersonCharacter CharRef))
  (Variables|/Game/ThirdPerson/Blueprints/BP_ThirdPersonCharacter.BP_ThirdPersonCharacter_C|SetIsOnRope? _asbp_third_person_character false)
  (Pawn|Components|CharacterMovement|SetMovementMode (Variables|/Script/Engine.Character|GetCharacterMovement _asbp_third_person_character) "MOVE_Walking" 0)
  (Transformation|SetActorRotation (Variables|Default|GetCharRef) (Math|Rotator|MakeRotator 0.0 0.0 (.yaw (Transformation|GetActorRotation (Variables|Default|GetCharRef)))))
  (bind _returnvalue (Physics|GetPhysicsLinearVelocity (Variables|Default|GetRope_Mesh) (Variables|Default|GetActiveRopeBone)))
  (Character|LaunchCharacter (Variables|Default|GetCharRef) (* _returnvalue 2.0) true true))

(fn ConstructionScript
  (bind _rope_mesh (Variables|Default|GetRope_Mesh))
  (for _index (range 0 (- (Class|SkinnedMeshComponent|GetNumBones (Variables|Default|GetRope_Mesh)) 1))
    (bind _returnvalue (AddComponent|AddBoxComponent false (Math|Transform|MakeTransform (- (Transformation|GetSocketLocation _rope_mesh (Class|SkinnedMeshComponent|GetBoneName _rope_mesh _index)) (Transformation|GetWorldLocation _rope_mesh)) "0, 0, 0" "1.000000,1.000000,1.000000")))
    (Utilities|Array|Add (Variables|Default|GetBoneBox) _returnvalue)))

(fn FindBestBone
  (bind _rope_mesh (Variables|Default|GetRope_Mesh))
  (for (_array_element _array_index) (Variables|Default|GetBoneBox)
    (if (> (Class|SkeletalMeshComponent|GetBoneMass _rope_mesh (Class|SkinnedMeshComponent|GetBoneName _rope_mesh _array_index) true) 0.0)
      (LocalVariables|SetCurrentIndex _array_index)
      (bind _output_get (LocalVariables|SetCurrentDistance (Math|Vector|Distance(Vector) (Transformation|GetWorldLocation _array_element) (Transformation|GetSocketLocation (Variables|/Script/Engine.Character|GetMesh (Variables|Default|GetCharRef)) "head"))))
      (if (or (< _output_get (LocalVariables|GetClosestDistance)) (< (LocalVariables|GetClosesIndex) 0))
        (LocalVariables|SetClosesIndex (LocalVariables|GetCurrentIndex))
        (LocalVariables|SetClosestDistance (LocalVariables|GetCurrentDistance)))))
  (return (LocalVariables|GetClosesIndex)))

(fn CanClimb?
  (params (ClimbDirection :type Float%20%28double-precision%29))
  (bind _rope_mesh (Variables|Default|GetRope_Mesh))
  (Development|PrintString (Utilities|String|ToString(Vector) (- (Transformation|GetSocketLocation _rope_mesh (Class|SkinnedMeshComponent|GetBoneName (Variables|Default|GetRope_Mesh) (Math|Integer|Clamp(Integer) (+ (Math|Float|Truncate (* ClimbDirection -7.0)) (Class|SkinnedMeshComponent|GetBoneIndex (Variables|Default|GetRope_Mesh) (Variables|Default|GetActiveRopeBone))) 37 93))) (Transformation|GetSocketLocation _rope_mesh (Variables|Default|GetActiveRopeBone)))))
  (if (!= (Variables|Default|GetActiveRopeBone) (Class|SkinnedMeshComponent|GetBoneName (Variables|Default|GetRope_Mesh) (Math|Integer|Clamp(Integer) (+ (Math|Float|Truncate (* ClimbDirection -7.0)) (Class|SkinnedMeshComponent|GetBoneIndex (Variables|Default|GetRope_Mesh) (Variables|Default|GetActiveRopeBone))) 37 93)))
    (bind _output_get (Variables|Default|SetActiveRopeBone (Class|SkinnedMeshComponent|GetBoneName (Variables|Default|GetRope_Mesh) (Math|Integer|Clamp(Integer) (+ (Math|Float|Truncate (* ClimbDirection -7.0)) (Class|SkinnedMeshComponent|GetBoneIndex (Variables|Default|GetRope_Mesh) (Variables|Default|GetActiveRopeBone))) 37 93))))
    (Development|PrintString (Utilities|String|ToString(Name) _output_get))
    (return true)
    (else
      (return false))))